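; BP_Sonu is a character Blueprint that snaps its facing between two opposite yaws and tracks death from damage.
; Tick picks yaw from velocity pitch at a 180-degree threshold, which normalized pitch never reaches, so it resolves to yaw 180.
; FlipToRotate flips by acceleration X sign but is not called here.
; GetHurt zeroes health and flags death on lethal damage, but never stores non-lethal damage.
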(event EventTick
  (params (DeltaSeconds :type Float%20%28single-precision%29))
  (bind _returnvalue (Pawn|GetController))
  (if (>= (.pitch (Math|Rotator|MakeRotfromX (Transformation|GetVelocity))) 1.8e+02)
    (Pawn|SetControlRotation _returnvalue (Math|Rotator|MakeRotator 0.0 0.0 0.0))
    (else
      (Pawn|SetControlRotation _returnvalue (Math|Rotator|MakeRotator 0.0 0.0 1.8e+02)))))

(fn ConstructionScript)

(fn GetHurt
  (params (Damage :type Float%20%28double-precision%29))
  (if (<= (- (Variables|Default|GetCurrentHealth) Damage) 0.0)
    (Variables|Default|SetCurrentHealth 0.0)
    (bind _output_get (Variables|Default|SetIsDead? true))
    (return _output_get)
    (else
      (bind _output_get_2 (Variables|Default|SetIsDead? false))
      (return _output_get_2))))

(fn FliptoRotate
  (bind _returnvalue (Pawn|GetController))
  (Math|Float|CompareFloat (.x (Pawn|Components|CharacterMovement|GetCurrentAcceleration (Variables|Character|GetCharacterMovement))) 0.0
    (:>
      (Pawn|SetControlRotation _returnvalue (Math|Rotator|MakeRotator 0.0 0.0 0.0)))
    (:<
      (Pawn|SetControlRotation _returnvalue (Math|Rotator|MakeRotator 0.0 0.0 1.8e+02)))))